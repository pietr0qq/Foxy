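; Shop actor that the player can interact with to open the shop screen.
; A box overlap shows an interaction prompt and enables the HUD's interact button while the player is in range, reversing both on exit.
; Interact calls OpenShop when IsOpen is false, which shows the cursor, adds a new ShopWidget and disables character input.
; IsOpen is never set here, and the UI-only input mode node is unconnected.
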(event OnComponentBeginOverlap(Box)
  (params (OverlappedComponent :type Primitive%20Component%20Object%20Reference) (OtherActor :type Actor%20Object%20Reference) (OtherComp :type Primitive%20Component%20Object%20Reference) (OtherBodyIndex :type Integer) (bFromSweep :type Boolean) (SweepResult :type Hit%20Result%20Structure%20%28by%20ref%29))
  (bind _returnvalue (Game|GetPlayerCharacter 0))
  (if (== OtherActor _returnvalue)
    (UserInterface|Viewport|AddtoViewport (Variables|Default|GetInteract%20widget) 0)
    (bind _asbp_player (Utilities|Casting|CastToBP_Player _returnvalue))
    (Utilities|IsValid (Variables|/Game/Blueprints/BP_Player.BP_Player_C|GetHUDRef _asbp_player)
      (:Is%20Valid
        (bind _ashud (Utilities|Casting|CastToHUD (Variables|/Game/Blueprints/BP_Player.BP_Player_C|GetHUDRef _asbp_player)))
        (Widget|SetIsEnabled (Variables|/Game/Maps/HUD/HUD.HUD_C|GetBtnInteract _ashud) true)))))

(event OnComponentEndOverlap(Box)
  (params (OverlappedComponent :type Primitive%20Component%20Object%20Reference) (OtherActor :type Actor%20Object%20Reference) (OtherComp :type Primitive%20Component%20Object%20Reference) (OtherBodyIndex :type Integer))
  (bind _returnvalue (Game|GetPlayerCharacter 0))
  (if (== _returnvalue OtherActor)
    (Widget|RemovefromParent (Variables|Default|GetInteract%20widget))
    (bind _asbp_player (Utilities|Casting|CastToBP_Player _returnvalue))
    (Utilities|IsValid (Variables|/Game/Blueprints/BP_Player.BP_Player_C|GetHUDRef _asbp_player)
      (:Is%20Valid
        (bind _ashud (Utilities|Casting|CastToHUD (Variables|/Game/Blueprints/BP_Player.BP_Player_C|GetHUDRef _asbp_player)))
        (Widget|SetIsEnabled (Variables|/Game/Maps/HUD/HUD.HUD_C|GetBtnInteract _ashud) false)))))

(event Custom|Open%20Shop
  (Variables|/Script/Engine.PlayerController|SetbShowMouseCursor (Game|GetPlayerController 0) true)
  (bind _returnvalue (UserInterface|CreateWidget "/Game/Blueprints/Shop/ShopWidget.ShopWidget_C"))
  (UserInterface|Viewport|AddtoViewport _returnvalue 0)
  (Input|DisableInput (Game|GetPlayerCharacter 0) 0))

(event EventBeginPlay
  (Rendering|Components|Sprite|SetSprite (Variables|Default|GetPaperSprite) (Variables|Default|GetShopSprite))
  (bind _returnvalue (UserInterface|CreateWidget "/Game/Blueprints/Shop/P_interact.P_interact_C"))
  (Variables|Default|SetInteract%20widget _returnvalue))

(fn ConstructionScript)

(fn Interact
  (params (Inteactor :type Character%20Object%20Reference))
  (if (not (Variables|Default|GetIs%20open))
    (CallFunction|OpenShop)
    (return true)))