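; Opossum enemy Blueprint for a 2D flipbook game that patrols and can either kill the player or be stomped.
; A timeline, with play rate set by Speed, lerps the sprite between Start and End and sets its X scale from a Rotation track.
; Body overlap calls Death on the GM game mode; head overlap plays the death flipbook and destroys the enemy.
; Disable flags, one reset after a short delay, keep each outcome from triggering the other.
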(event OnComponentBeginOverlap(Body)
  (params (OverlappedComponent :type Primitive%20Component%20Object%20Reference) (OtherActor :type Actor%20Object%20Reference) (OtherComp :type Primitive%20Component%20Object%20Reference) (OtherBodyIndex :type Integer) (bFromSweep :type Boolean) (SweepResult :type Hit%20Result%20Structure%20%28by%20ref%29))
  (Utilities|Casting|CastToBP_Player OtherActor)
  (if (not (Variables|Default|GetDisableKillPlayer))
    (bind _asgm (Utilities|Casting|CastToGM (Game|GetGameMode)))
    (Default|Death _asgm)
    (Variables|Default|SetDisableKillEnemy true)
    (Utilities|FlowControl|Delay 0.7)
    (Variables|Default|SetDisableKillEnemy false)))

(event OnComponentBeginOverlap(Head)
  (params (OverlappedComponent :type Primitive%20Component%20Object%20Reference) (OtherActor :type Actor%20Object%20Reference) (OtherComp :type Primitive%20Component%20Object%20Reference) (OtherBodyIndex :type Integer) (bFromSweep :type Boolean) (SweepResult :type Hit%20Result%20Structure%20%28by%20ref%29))
  (bind _opossum (Variables|Default|Getopossum))
  (bind _returnvalue (Transformation|GetWorldScale _opossum))
  (Utilities|Casting|CastToBP_Player OtherActor)
  (if (not (Variables|Default|GetDisableKillEnemy))
    (Variables|Default|SetDisableKillPlayer true)
    (CallFunction|EnemyDeath)
    (bind (_direction _floattrack _rotation) (Timeline|MovementTimeline Stop)
      (:Update
        (Transformation|SetRelativeLocation (Variables|Default|Getopossum) (Math|Vector|Lerp(Vector) (Variables|Default|GetStart) (Variables|Default|GetEnd) _floattrack) false false)
        (Transformation|SetWorldScale3D _opossum (Math|Vector|MakeVector _rotation (.y _returnvalue) (.z _returnvalue)))))))

(event Custom|EnemyDeath
  (Sprite|SetFlipbook (Variables|Default|Getopossum) "/Game/PNG/sprites/enemy-death/death.death")
  (Utilities|FlowControl|Delay 0.5)
  (Actor|DestroyActor))

(event Custom|CustomEvent
  (params (DeltaSeconds :type Float%20%28single-precision%29)))

(event EventBeginPlay
  (bind _opossum (Variables|Default|Getopossum))
  (bind _returnvalue (Transformation|GetWorldScale _opossum))
  (Components|Timeline|SetPlayRate (Variables|Default|GetMovementTimeline) (Variables|Default|GetSpeed))
  (bind (_direction _floattrack _rotation) (Timeline|MovementTimeline Play)
    (:Update
      (Transformation|SetRelativeLocation (Variables|Default|Getopossum) (Math|Vector|Lerp(Vector) (Variables|Default|GetStart) (Variables|Default|GetEnd) _floattrack) false false)
      (Transformation|SetWorldScale3D _opossum (Math|Vector|MakeVector _rotation (.y _returnvalue) (.z _returnvalue))))))

(fn ConstructionScript)