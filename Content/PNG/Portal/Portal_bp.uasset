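; Portal actor that ends the current level and loads the next one when the player overlaps its box.
; On overlap it plays a level-passed sound, clears all widgets, shows a loading screen, then opens the referenced Level after short delays.
; It copies Hearts from the GM game mode to GameLevelInstance right after the open-level call, carrying them across levels.
; A switch on LevelID is left unconnected.
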(event OnComponentBeginOverlap(Box)
  (params (OverlappedComponent :type Primitive%20Component%20Object%20Reference) (OtherActor :type Actor%20Object%20Reference) (OtherComp :type Primitive%20Component%20Object%20Reference) (OtherBodyIndex :type Integer) (bFromSweep :type Boolean) (SweepResult :type Hit%20Result%20Structure%20%28by%20ref%29))
  (Utilities|Casting|CastToBP_Player OtherActor)
  (bind _asgm (Utilities|Casting|CastToGM (Game|GetGameMode)))
  (Audio|PlaySound2D "/Game/Sound_Music/LevelPassed.LevelPassed" 1.0 1.0 0.0 0 0)
  (Utilities|FlowControl|Delay 0.2)
  (Viewport|RemoveAllWidgets)
  (bind _returnvalue (UserInterface|CreateWidget "/Game/Maps/Loading/LoadingScreen.LoadingScreen_C"))
  (UserInterface|Viewport|AddtoViewport _returnvalue 0)
  (Utilities|FlowControl|Delay 1.0)
  (Utilities|Casting|CastToBP_Player (Game|GetPlayerCharacter 0))
  (Game|OpenLevel(byObjectReference) (Variables|Default|GetLevel))
  (bind _asgame_level_instance (Utilities|Casting|CastToGameLevelInstance (Game|GetGameInstance)))
  (Variables|/Game/Blueprints/GameLevelInstance.GameLevelInstance_C|SetHearts _asgame_level_instance (Variables|/Game/Blueprints/GM.GM_C|GetHearts _asgm)))

(fn ConstructionScript)